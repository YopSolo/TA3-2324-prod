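; BP_Spline2 is a construction-time spline tool that fills a spline with evenly spaced static mesh components.
; Its construction script advances a running distance by SizeCm, adding a mesh at that point's local, unscaled spline transform until the length is covered.
; Each mesh gets an extra 90-degree local rotation on top of the spline's orientation.
; The distance increments before each placement, and the event graph holds no active logic.
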(fn `UserConstructionScript`
  (while (< (`self.totalDistanceCm`) (- (`SplineComponent.GetSplineLength` (`self.Spline`)) (`self.sizeCm`)))
    (bind _output_get (set `self.totalDistanceCm` (+ (`self.totalDistanceCm`) (`self.sizeCm`))))
    (bind _returnvalue (`AddComponent|NODE_AddStaticMeshComponent-0` :`RelativeTransform` (`SplineComponent.GetTransformAtDistanceAlongSpline` (`self.Spline`) _output_get "Local" false)))
    (`SceneComponent.K2_AddLocalRotation` _returnvalue (struct :`Yaw` 90.0) false false)))