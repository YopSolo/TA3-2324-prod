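; BP_Tower is a Blueprint that procedurally builds a tower wall as a flat grid of meshes in its Construction Script.
; Nested loops place rotated instances at fixed spacing along X and Z, using a running counter's parity to alternate between two Instanced Static Mesh components.
; A disconnected alternative builds a similar grid from individual Static Mesh components spaced by their bounds, but it never runs.
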(fn `UserConstructionScript`
  ;[0 0 0] instantiated static mesh
  (for _index (range 26)
    (for _index_2 (range 44)
      (bind _result (`/Engine/EditorBlueprintResources/StandardMacros.IncrementInt` (`self.count`))
        (:`  `
          (if (== (mod _result 2) 0)
            (`InstancedStaticMeshComponent.AddInstance` (`self.InstancedStaticMesh`) (`KismetMathLibrary.MakeTransform` (`KismetMathLibrary.MakeVector` (`KismetMathLibrary.Conv_IntToDouble` (* 300 _index_2)) 0.0 (`KismetMathLibrary.Conv_IntToDouble` (* _index 300))) (struct :`Yaw` 90.0)) false)
            (else
              (`InstancedStaticMeshComponent.AddInstance` (`self.InstancedStaticMesh2`) (`KismetMathLibrary.MakeTransform` (`KismetMathLibrary.MakeVector` (`KismetMathLibrary.Conv_IntToDouble` (* 300 _index_2)) 0.0 (`KismetMathLibrary.Conv_IntToDouble` (* 300 _index))) (struct :`Yaw` 90.0)) false))))))))